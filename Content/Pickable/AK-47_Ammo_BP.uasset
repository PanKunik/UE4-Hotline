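; AK-47 ammo pickup actor that refills the top-down character's AK ammo when the character overlaps it.
; On overlap it casts to TopDownCharacter and does nothing if the ammo is already full.
; Otherwise it adds the box's Ammo, capped at the character's maximum, and destroys itself, discarding any surplus.
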(event EventBeginPlay)

(event Collision|EventActorBeginOverlap
  (params (OtherActor :type Actor%20Object%20Reference))
  (bind _astop_down_character (Utilities|Casting|CastToTopDownCharacter OtherActor))
  (if (< (Variables|/Game/TopDownBP/Blueprints/TopDownCharacter.TopDownCharacter_C|GetAK_Ammo _astop_down_character) (Variables|/Game/TopDownBP/Blueprints/TopDownCharacter.TopDownCharacter_C|GetAK_MaxAmmo _astop_down_character)) ; Czy brakuje amunicji?
    (if (> (- (Variables|/Game/TopDownBP/Blueprints/TopDownCharacter.TopDownCharacter_C|GetAK_MaxAmmo _astop_down_character) (Variables|/Game/TopDownBP/Blueprints/TopDownCharacter.TopDownCharacter_C|GetAK_Ammo _astop_down_character)) (Variables|Default|GetAmmo)) ; Czy brak więcej, niż jest w pudełku?
      (Variables|/Game/TopDownBP/Blueprints/TopDownCharacter.TopDownCharacter_C|SetAK_Ammo _astop_down_character (+ (Variables|Default|GetAmmo) (Variables|/Game/TopDownBP/Blueprints/TopDownCharacter.TopDownCharacter_C|GetAK_Ammo _astop_down_character)))
      (Actor|DestroyActor)
      (else
        (Variables|/Game/TopDownBP/Blueprints/TopDownCharacter.TopDownCharacter_C|SetAK_Ammo _astop_down_character (Variables|/Game/TopDownBP/Blueprints/TopDownCharacter.TopDownCharacter_C|GetAK_MaxAmmo _astop_down_character))
        (Actor|DestroyActor)))))

(event EventTick
  (params (DeltaSeconds :type Float%20%28single-precision%29)))

(fn ConstructionScript)