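; Wardrobe actor whose two doors the player can open and close when nearby.
; Its trigger toggles the HUD prompt and an availability flag, which lets Tick register the wardrobe with the character through CanInteract.
; Interact hides the prompt and plays or reverses a timeline that rotates the doors in mirrored yaw.
; When the timeline finishes, it flips the closed state and restores the prompt if the player remains in range.
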(event OnComponentBeginOverlap(Trigger)
  (params (OverlappedComponent :type Primitive%20Component%20Object%20Reference) (OtherActor :type Actor%20Object%20Reference) (OtherComp :type Primitive%20Component%20Object%20Reference) (OtherBodyIndex :type Integer) (bFromSweep :type Boolean) (SweepResult :type Hit%20Result%20Structure%20%28by%20ref%29))
  ;[1 1 1] Check if player started overlaping
  (if (Utilities|Enum|Equal(Enum) (Utilities|GetObjectName OtherActor) (Utilities|GetObjectName (Game|GetPlayerCharacter 0)))
    (Variables|Default|SetCanDoAction true)
    (bind _ashud_bp (Utilities|Casting|CastToHUD_BP (HUD|GetHUD (Game|GetPlayerController 0))))
    (Default|DisplayText _ashud_bp true)))

(event OnComponentEndOverlap(Trigger)
  (params (OverlappedComponent :type Primitive%20Component%20Object%20Reference) (OtherActor :type Actor%20Object%20Reference) (OtherComp :type Primitive%20Component%20Object%20Reference) (OtherBodyIndex :type Integer))
  ;[1 1 1] Check if player ended overlaping
  (if (Utilities|Enum|Equal(Enum) (Utilities|GetObjectName OtherActor) (Utilities|GetObjectName (Game|GetPlayerCharacter 0)))
    (Variables|Default|SetCanDoAction false)
    (bind _ashud_bp (Utilities|Casting|CastToHUD_BP (HUD|GetHUD (Game|GetPlayerController 0))))
    (Default|DisplayText _ashud_bp false)))

(event Custom|Interact
  ;[1 1 1] Interact with wardrobe (open or close)
  (if (Variables|Default|GetClosed)
    (bind _ashud_bp (Utilities|Casting|CastToHUD_BP (HUD|GetHUD (Game|GetPlayerController 0))))
    (Default|DisplayText _ashud_bp false)
    (bind _newtrack_0 (Timeline|Open%20Wardrobe Play)
      (:Update
        (Transformation|SetRelativeRotation (Variables|Default|GetLeftDoor) (Math|Rotator|MakeRotator 0.0 0.0 _newtrack_0) false false)
        (Transformation|SetRelativeRotation (Variables|Default|GetRightDoor) (Math|Rotator|MakeRotator 0.0 0.0 (- 0.0 _newtrack_0)) false false))
      (:Finished
        (if (Variables|Default|GetClosed)
          (Variables|Default|SetClosed false)
          (else
            (Variables|Default|SetClosed true)))
        (if (Variables|Default|GetCanDoAction)
          (bind _ashud_bp_2 (Utilities|Casting|CastToHUD_BP (HUD|GetHUD (Game|GetPlayerController 0))))
          (Default|DisplayText _ashud_bp_2 true))))
    (else
      (bind _ashud_bp_3 (Utilities|Casting|CastToHUD_BP (HUD|GetHUD (Game|GetPlayerController 0))))
      (Default|DisplayText _ashud_bp_3 false)
      (Timeline|Open%20Wardrobe Reverse))))

(event EventBeginPlay)

(event Collision|EventActorBeginOverlap
  (params (OtherActor :type Actor%20Object%20Reference)))

(event EventTick
  (params (DeltaSeconds :type Float%20%28single-precision%29))
  ;[1 1 1] Check if player is still in trigger
  (if (Variables|Default|GetCanDoAction)
    (bind _astop_down_character (Utilities|Casting|CastToTopDownCharacter (stale OnComponentBeginOverlap(Trigger) OtherActor)))
    (Default|CanInteract _astop_down_character self)))

(fn ConstructionScript)