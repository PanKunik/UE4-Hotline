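; AK-47 pickup actor that grants the weapon to the TopDownCharacter.
; On overlap it casts to that character, sets its HasAK flag and destroys itself.
; A separate Reload function, not called in this graph, tops up InClip to ClipSize from the Ammo reserve, or moves whatever remains when the reserve runs short.
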(event EventBeginPlay)

(event Collision|EventActorBeginOverlap
  (params (OtherActor :type Actor%20Object%20Reference))
  (bind _astop_down_character (Utilities|Casting|CastToTopDownCharacter OtherActor))
  (if true
    (Variables|/Game/TopDownBP/Blueprints/TopDownCharacter.TopDownCharacter_C|SethasAK _astop_down_character true)
    (Actor|DestroyActor)))

(event EventTick
  (params (DeltaSeconds :type Float%20%28single-precision%29)))

(fn ConstructionScript)

(fn Reload
  (if (not (== (Variables|Default|GetInClip) (Variables|Default|GetClipSize))) ; Czy w magazynku nie brakuje amunicji?
    (if (< (- (Variables|Default|GetClipSize) (Variables|Default|GetInClip)) (Variables|Default|GetAmmo)) ; Czy masz naboje do uzupełnienia magazynka?
      (Variables|Default|SetAmmo (- (Variables|Default|GetAmmo) (- (Variables|Default|GetClipSize) (Variables|Default|GetInClip)))) ; Odejmij naboje uzupełnione do magazynka
      (Variables|Default|SetInClip (Variables|Default|GetClipSize)) ; Napełnij magazynek
      (else
        (Variables|Default|SetInClip (+ (Variables|Default|GetInClip) (Variables|Default|GetAmmo))) ; Dodaj resztę naboi
        (Variables|Default|SetAmmo 0) ; Brak naboji w zapasie
      ))))