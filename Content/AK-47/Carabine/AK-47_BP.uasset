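; AK-47 weapon actor that handles firing, ammo checks and reloading.
; Shoot decrements the clip, spawns a damage-carrying bullet and a randomly deflected shell casing from mesh sockets, aligned to the instigator's rotation, plus muzzle flash and sound.
; Separate check events set the CanShoot and CanReload flags from reload state, clip and reserve ammo.
; Reload tops up the clip from reserve ammo, using whatever remains when short.
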(event Custom|Check%20if%20can%20shoot
  ;[1 1 1] Check if can shoot
  (if (Variables|Default|GetisReloading)
    (Variables|Default|SetCanShoot false :!label _label)
    (elif (> (Variables|Default|GetInClip) 0)
      (Variables|Default|SetCanShoot true)
      (else
        (goto _label)))))

(event Custom|Check%20if%20can%20reload
  ;[1 1 1] Check if can reload
  (if (> (Variables|Default|GetClipSize) (Variables|Default|GetInClip))
    (if (> (Variables|Default|GetAmmo) 0)
      (Variables|Default|SetCanReload true)
      (else
        (Variables|Default|SetCanReload false :!label _label)))
    (else
      (goto _label))))

(event Custom|Shoot
  (bind _returnvalue (Game|GetInstigator))
  (bind _ak_47 (Variables|Default|GetAK-47))
  (bind _returnvalue_2 (Transformation|GetActorRotation _returnvalue))
  (bind _returnvalue_3 (Transformation|GetSocketLocation _ak_47 "BulletPos"))
  (bind _returnvalue_4 (Transformation|GetActorRotation _returnvalue))
  (bind _returnvalue_5 (Math|Vector|GetForwardVector _returnvalue_4))
  (bind _returnvalue_6 (+ _returnvalue_3 _returnvalue_5))
  (bind _returnvalue_7 (Math|Transform|MakeTransform _returnvalue_6 _returnvalue_4))
  (bind (_location _rotation) (Math|Transform|BreakTransform _returnvalue_7))
  ;[1 1 1] Shoot
  (Variables|Default|SetInClip (- (Variables|Default|GetInClip) 1))
  (bind _returnvalue_8 (Game|SpawnActorfromClass "/Game/AK-47/Bullets/7-62x39mm_Bullet_Blueprint.7-62x39mm_Bullet_Blueprint_C" _returnvalue_7 "Undefined" 0 (Game|GetInstigator)))
  (Default|SetDamage _returnvalue_8 (Variables|Default|GetDamage))
  (bind _returnvalue_9 (Game|SpawnActorfromClass "/Game/AK-47/Bullets/7-62x39mm_Shell_Blueprint.7-62x39mm_Shell_Blueprint_C" (Math|Transform|MakeTransform (+ (Transformation|GetSocketLocation (Variables|Default|GetAK-47) "ShellPos") (Math|Vector|GetForwardVector _returnvalue_2)) _returnvalue_2) "Undefined" 0 0))
  (Variables|/Script/Engine.MovementComponent|SetVelocity (Variables|/Game/AK-47/Bullets/7-62x39mm_Shell_Blueprint.7-62x39mm_Shell_Blueprint_C|GetProjectileMovement _returnvalue_9) (Math|Vector|RotateVector (Transformation|GetVelocity _returnvalue_9) (Math|Rotator|MakeRotator 0.0 0.0 (Math|Random|RandomFloatinRange -15.0 15.0))))
  (Transformation|SetActorRotation _returnvalue_9 (Math|Rotator|MakeRotator (.Roll (Math|Rotator|BreakRotator (Transformation|GetActorRotation _returnvalue_9))) (.Pitch (Math|Rotator|BreakRotator (Transformation|GetActorRotation _returnvalue_9))) (+ (.Yaw (Math|Rotator|BreakRotator (Transformation|GetActorRotation _returnvalue_9))) (Math|Random|RandomFloatinRange -3e+01 3e+01))))
  (bind _returnvalue_10 (Effects|SpawnEmitteratLocation "/Game/SFX/P_MuzzleFlash.P_MuzzleFlash" _location _rotation))
  (Audio|PlaySoundatLocation "/Game/SFX/Sounds/AK_47_shoot_CSGO_Sound_Effect.AK_47_shoot_CSGO_Sound_Effect" (Transformation|GetWorldLocation _returnvalue_10) "0, 0, 0" 1.0 1.0 0.0 (Variables|Default|GetAttenuation)))

(event EventBeginPlay)

(event Collision|EventActorBeginOverlap
  (params (OtherActor :type Actor%20Object%20Reference)))

(event EventTick
  (params (DeltaSeconds :type Float%20%28single-precision%29)))

(fn ConstructionScript)

(fn Reload
  (if (not (== (Variables|Default|GetInClip) (Variables|Default|GetClipSize))) ; Czy w magazynku nie brakuje amunicji?
    (if (< (- (Variables|Default|GetClipSize) (Variables|Default|GetInClip)) (Variables|Default|GetAmmo)) ; Czy masz naboje do uzupełnienia magazynka?
      (Variables|Default|SetAmmo (- (Variables|Default|GetAmmo) (- (Variables|Default|GetClipSize) (Variables|Default|GetInClip)))) ; Odejmij naboje uzupełnione do magazynka
      (Variables|Default|SetInClip (Variables|Default|GetClipSize)) ; Napełnij magazynek
      (else
        (Variables|Default|SetInClip (+ (Variables|Default|GetInClip) (Variables|Default|GetAmmo))) ; Dodaj resztę naboi
        (Variables|Default|SetAmmo 0) ; Brak naboji w zapasie
      ))))