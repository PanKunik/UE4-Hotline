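; Main menu actor that creates and shows the main menu widget when play begins.
; BeginPlay adds the widget to the viewport with a crosshair cursor.
; If the saved window mode is fullscreen, it checks the widget's fullscreen box, loads its resolution options, and applies the desktop resolution through GameUserSettings.
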(event EventBeginPlay
  (bind _returnvalue (UserInterface|CreateWidget "/Game/MainMenu/MainMenu_Widget.MainMenu_Widget_C"))
  (UserInterface|Viewport|AddtoViewport _returnvalue 0)
  (Class|Widget|SetCursor _returnvalue "Crosshairs")
  (bind _returnvalue_2 (Settings|GetGameUserSettings))
  (if (Utilities|Enum|Equal(Enum) (Utilities|String|EnumtoString (Class|GameUserSettings|GetFullscreenMode _returnvalue_2)) "Fullscreen")
    (Class|CheckBox|SetIsChecked (Variables|/Game/MainMenu/MainMenu_Widget.MainMenu_Widget_C|GetFullscreenMode _returnvalue) true)
    (Default|LoadResolution _returnvalue true)
    (Class|GameUserSettings|SetScreenResolution _returnvalue_2 (Class|GameUserSettings|GetDesktopResolution _returnvalue_2))
    (Class|GameUserSettings|ApplyResolutionSettings _returnvalue_2 false)))

(event Collision|EventActorBeginOverlap
  (params (OtherActor :type Actor%20Object%20Reference)))

(event EventTick
  (params (DeltaSeconds :type Float%20%28single-precision%29)))

(fn ConstructionScript)